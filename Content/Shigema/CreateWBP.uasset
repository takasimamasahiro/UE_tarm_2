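; CreateWBP is a trigger actor that shows the clear screen when the first-person player character enters its Box.
; The overlap checks the other actor against BP_FirstPersonCharacter, calls ShowWidget, then destroys that character.
; ShowWidget creates WBP_ClearScreen, stores it and adds it to the viewport, guarded by IsWidgetVisible against duplicates.
; ToggleWidgetVisibility is empty, and leftover show/hide toggle logic is disconnected.
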(event OnComponentBeginOverlap(Box)
  (params (OverlappedComponent :type Primitive%20Component%20Object%20Reference) (OtherActor :type Actor%20Object%20Reference) (OtherComp :type Primitive%20Component%20Object%20Reference) (OtherBodyIndex :type Integer) (bFromSweep :type Boolean) (SweepResult :type Hit%20Result%20Structure%20%28by%20ref%29))
  (bind _returnvalue (Actor|GetActorOfClass "/Game/FirstPerson/Blueprints/BP_FirstPersonCharacter.BP_FirstPersonCharacter_C"))
  (if (== OtherActor _returnvalue)
    (CallFunction|ShowWidget)
    (bind _returnvalue_2 (Actor|GetActorOfClass "/Game/FirstPerson/Blueprints/BP_FirstPersonCharacter.BP_FirstPersonCharacter_C"))
    (Actor|DestroyActor _returnvalue_2)))

(event Custom|ToggleWidgetVisibility
  ;[1 1 1] クリア画面の表示非表示
)

(event Custom|ShowWidget
  (if (not (Variables|Default|GetIsWidgetVisible))
    (bind _returnvalue (UserInterface|CreateWidget "/Game/Shigema/WBP_ClearScreen.WBP_ClearScreen_C"))
    (Variables|Default|SetClearWidgetInstance _returnvalue)
    (UserInterface|Viewport|AddtoViewport _returnvalue 0)
    (Variables|Default|SetIsWidgetVisible true)))

(event EventBeginPlay)

(event Collision|EventActorBeginOverlap
  (params (OtherActor :type Actor%20Object%20Reference)))

(event EventTick
  (params (DeltaSeconds :type Float%20%28single-precision%29)))

(fn ConstructionScript)